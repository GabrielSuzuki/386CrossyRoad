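; Player chicken Character that hops between lanes in a Crossy Road-style game, dying when hit by cars or trains or straying too far sideways.
; Four input axes launch it and turn the mesh through Timelines.
; A DoOnce cooldown blocks input during each hop, then shifts mesh and camera by the measured travel.
; Tick pushes it down while alive and slides it by Deadspeed when dead; vehicle hits squash it, but their Deadspeed assignments are disconnected.
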(event `self.ReceiveTick`
  (params (DeltaSeconds :type "Float (single-precision)"))
  (bind (_returnvalue_x _returnvalue_y) (`KismetMathLibrary.BreakVector` (`self.K2_GetActorLocation`)))
  (if (`self.isDead`)
    (`self.K2_AddActorWorldOffset` (`KismetMathLibrary.MakeVector` 0.0 (* (`self.deadspeed`) DeltaSeconds)))
    (set `self.canmove` false)
    (elif (> (`KismetMathLibrary.Abs` _returnvalue_y) 500.0)
      (set `self.isDead` true)
      (else
        (`self.K2_AddActorWorldOffset` (0.0 0.0 -4.0))))))

(event `InputAxis|ForwardMovement`
  (params (AxisValue :type "Float (single-precision)"))
  (bind _staticmesh (`self.StaticMesh`))
  (if (and (`self.canmove`) (> (`KismetMathLibrary.Abs` AxisValue) 0.3))
    (`self.MovementCooldown`)
    (`self.LaunchCharacter` (`KismetMathLibrary.MakeVector` (* AxisValue 150.0) 0.0 500.0) true true)
    (bind (_direction _newtrack_0) (`Timeline|Timeline_0` :!via `PlayFromStart`)
      (:`Update`
        (`SceneComponent.K2_SetWorldRotation` _staticmesh (`KismetMathLibrary.RLerp` (`SceneComponent.K2_GetComponentRotation` _staticmesh) (struct :`Yaw` -180.0) _newtrack_0 true) false false)))))

(event `InputAxis|BackMovement`
  (params (AxisValue :type "Float (single-precision)"))
  (bind _staticmesh (`self.StaticMesh`))
  (if (and (`self.canmove`) (> (`KismetMathLibrary.Abs` AxisValue) 0.3))
    (`self.MovementCooldown`)
    (`self.LaunchCharacter` (`KismetMathLibrary.MakeVector` (* AxisValue 150.0) 0.0 500.0) true true)
    (bind (_direction _newtrack_0) (`Timeline|Timeline_1` :!via `PlayFromStart`)
      (:`Update`
        (`SceneComponent.K2_SetWorldRotation` _staticmesh (`KismetMathLibrary.RLerp` (`SceneComponent.K2_GetComponentRotation` _staticmesh) (struct) _newtrack_0 true) false false)))))

(event `InputAxis|RightMovement`
  (params (AxisValue :type "Float (single-precision)"))
  (bind _staticmesh (`self.StaticMesh`))
  (if (and (`self.canmove`) (> (`KismetMathLibrary.Abs` AxisValue) 0.3))
    (`self.MovementCooldown`)
    (`self.LaunchCharacter` (`KismetMathLibrary.MakeVector` 0.0 (* AxisValue 150.0) 500.0) true true)
    (bind (_direction _newtrack_0) (`Timeline|Timeline_2` :!via `PlayFromStart`)
      (:`Update`
        (`SceneComponent.K2_SetWorldRotation` _staticmesh (`KismetMathLibrary.RLerp` (`SceneComponent.K2_GetComponentRotation` _staticmesh) (struct :`Yaw` -90.0) _newtrack_0 true) false false)))))

(event `InputAxis|LeftMovement`
  (params (AxisValue :type "Float (single-precision)"))
  (bind _staticmesh (`self.StaticMesh`))
  (if (and (`self.canmove`) (> (`KismetMathLibrary.Abs` AxisValue) 0.3))
    (`self.MovementCooldown`)
    (`self.LaunchCharacter` (`KismetMathLibrary.MakeVector` 0.0 (* AxisValue 150.0) 500.0) true true)
    (bind (_direction _newtrack_0) (`Timeline|Timeline_3` :!via `PlayFromStart`)
      (:`Update`
        (`SceneComponent.K2_SetWorldRotation` _staticmesh (`KismetMathLibrary.RLerp` (`SceneComponent.K2_GetComponentRotation` _staticmesh) (struct :`Yaw` 90.0) _newtrack_0 true) false false)))))

(event `MovementCooldown`
  (bind _staticmesh (`self.StaticMesh`))
  (bind _camera (`self.Camera`))
  (bind _currentmovement_x (`KismetMathLibrary.BreakVector` (`self.currentMovement`)))
  (bind _aftermovement_x (`KismetMathLibrary.BreakVector` (`self.afterMovement`)))
  (bind _output_get (set `self.currentMovement` (`self.K2_GetActorLocation`)))
  (`/Engine/EditorBlueprintResources/StandardMacros.DoOnce` false :!label _label
    (:`Completed`
      (set `self.canmove` false)
      (`KismetSystemLibrary.Delay` 0.7)
      (bind _output_get_2 (set `self.afterMovement` (`self.K2_GetActorLocation`)))
      (set `self.canmove` true)
      (bind _returnvalue (`KismetMathLibrary.Vector_Distance` _output_get_2 _output_get))
      (`KismetSystemLibrary.PrintString` (`KismetStringLibrary.Conv_DoubleToString` _returnvalue))
      (if (> _aftermovement_x (+ _currentmovement_x 5.0))
        (if (< _returnvalue 80.0)
          (bind _returnvalue_2 (* _returnvalue -1.0))
          (`SceneComponent.K2_AddRelativeLocation` _staticmesh (`KismetMathLibrary.MakeVector` _returnvalue_2) false false)
          (`SceneComponent.K2_AddRelativeLocation` _camera (`KismetMathLibrary.MakeVector` _returnvalue_2) false false)
          (goto _label :!via `Reset`)
          (elif (> _returnvalue 80.0)
            (bind _returnvalue_3 (- _returnvalue 80.0))
            (`KismetSystemLibrary.PrintString` (`KismetStringLibrary.Conv_DoubleToString` _returnvalue_3))
            (`SceneComponent.K2_AddRelativeLocation` _staticmesh (`KismetMathLibrary.MakeVector` _returnvalue_3) false false)
            (`SceneComponent.K2_AddRelativeLocation` _camera (`KismetMathLibrary.MakeVector` _returnvalue_3) false false)
            (goto _label :!via `Reset`)
            (else
              (goto _label :!via `Reset`))))
        (elif true
          (`SceneComponent.K2_AddRelativeLocation` _staticmesh (`KismetMathLibrary.MakeVector` 0.0 _returnvalue_2) false false)
          (`SceneComponent.K2_AddRelativeLocation` _camera (`KismetMathLibrary.MakeVector` 0.0 _returnvalue_2) false false)
          (goto _label :!via `Reset`)
          (elif true
            (`SceneComponent.K2_AddRelativeLocation` _staticmesh (`KismetMathLibrary.MakeVector` 0.0 _returnvalue_3) false false)
            (`SceneComponent.K2_AddRelativeLocation` _camera (`KismetMathLibrary.MakeVector` 0.0 _returnvalue_3) false false)
            (goto _label :!via `Reset`)
            (else
              (goto _label :!via `Reset`))))))))

(event `self.Box.OnComponentBeginOverlap`
  (params (OverlappedComponent :type "PrimitiveComponent Object Reference") (OtherActor :type "Actor Object Reference") (OtherComp :type "PrimitiveComponent Object Reference") (OtherBodyIndex :type Integer) (bFromSweep :type Boolean) (SweepResult :type "HitResult Structure (by ref)"))
  (bind _asbp_cars (cast `/Game/Blueprints/bp_cars` OtherActor)
    (:`then`
      (set `self.isDead` true)
      (`self.K2_AddActorLocalTransform` (`KismetMathLibrary.MakeTransform` (0.0 0.0 0.0) (struct) (0.2 1.0 1.0))))
    (:`CastFailed`
      (bind _asbp_train (cast `/Game/Blueprints/bp_train` OtherActor))
      (set `self.isDead` true)
      (`self.K2_AddActorLocalTransform` (`KismetMathLibrary.MakeTransform` (0.0 0.0 0.0) (struct) (0.2 1.0 1.0))))))

(event `self.Box.OnComponentEndOverlap`
  (params (OverlappedComponent :type "PrimitiveComponent Object Reference") (OtherActor :type "Actor Object Reference") (OtherComp :type "PrimitiveComponent Object Reference") (OtherBodyIndex :type Integer))
  (cast `/Game/Blueprints/bp_lane` OtherActor))

(fn `UserConstructionScript`)