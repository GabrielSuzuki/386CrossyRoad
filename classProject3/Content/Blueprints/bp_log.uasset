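; Moving log actor that travels along world Y and is destroyed based on the player's progress along X.
; On BeginPlay it stores its start position and randomly picks a long or short log mesh.
; Each Tick it moves by ForwardSpeed and snaps back to the start once it exceeds Distance, creating a looping lane.
; It destroys itself when the player pawn's X plus DestroyBuffer exceeds its own X.
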(event `self.ReceiveBeginPlay`
  (set `self.StartPosition` (`self.K2_GetActorLocation`))
  (`StaticMeshComponent.SetStaticMesh` (`self.StaticMesh`) (select `int` (`KismetMathLibrary.RandomIntegerInRange` 0 1) :`0` "/Game/nature/long_log.long_log" :`1` "/Game/nature/short_log.short_log" :!type "StaticMesh Object Reference")))

(event `self.ReceiveTick`
  (params (DeltaSeconds :type "Float (single-precision)"))
  (bind _returnvalue_x (`KismetMathLibrary.BreakVector` (`self.K2_GetActorLocation`)))
  (bind _returnvalue_x_2 (`KismetMathLibrary.BreakVector` (`self.K2_GetActorLocation` (`GameplayStatics.GetPlayerPawn` 0))))
  (if (> (+ _returnvalue_x_2 (`self.DestroyBuffer`)) _returnvalue_x)
    (`self.K2_DestroyActor`)
    (else
      (`self.K2_AddActorWorldOffset` (`KismetMathLibrary.MakeVector` 0.0 (* DeltaSeconds (`self.ForwardSpeed`))))
      (if (> (`KismetMathLibrary.Vector_Distance` (`self.K2_GetActorLocation`) (`self.StartPosition`)) (`self.Distance`))
        (`self.K2_SetActorLocation` (`self.StartPosition`))))))

(fn `UserConstructionScript`)