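; Lane spawner for a Crossy Road-style game that builds a chain of randomly typed lanes along X, limited to a buffer ahead of the player.
; BeginPlay lays the initial strip, opening with type-0 lanes, each attached at the previous lane's SpawnPoint.
; SpawnLane scatters trees, rocks, coins or lilypads by lane type.
; Helper functions, not called here, spawn cars, trains and logs at either end of the newest lane.
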(event `self.ReceiveBeginPlay`
  (set `self.LaneState` 0)
  (`self.SpawnInitialLanes`))

(event `self.ReceiveTick`
  (params (DeltaSeconds :type "Float (single-precision)")))

(fn `SpawnCar`
  (params (SpawnLocation :type "Vector Structure"))
  (bind _returnvalue (`|SpawnActorFromClass` "/Game/Blueprints/bp_cars.bp_cars_C" (`KismetMathLibrary.MakeTransform` SpawnLocation) "Undefined" "OverrideRootScale" null null))
  (bind _output_get (set `self.NewestCar` _returnvalue))
  (set `/Game/Blueprints/bp_cars.CarsSpawner` self _output_get)
  (`StaticMeshComponent.SetStaticMesh` (`/Game/Blueprints/bp_cars.StaticMesh` _output_get) (select `int` (`KismetMathLibrary.RandomIntegerInRange` 0 4) :`0` "/Game/vehicle/police_car.police_car" :`1` "/Game/vehicle/truck.truck" :`2` "/Game/vehicle/yellow_short_car.yellow_short_car" :`3` "/Game/vehicle/fedex.fedex" :!type "StaticMesh Object Reference")))

(fn `SpawnCarAtSpawnPoint`
  (bind _newestcar (`self.NewestCar`))
  (bind _newestlane (`self.NewestLane`))
  (bind _carspawnpoint2 (`/Game/Blueprints/bp_lane.CarSpawnPoint2` _newestlane))
  (bind _returnvalue (select `int` (`KismetMathLibrary.RandomIntegerInRange` 0 1) :`0` (`/Game/Blueprints/bp_lane.CarSpawnPoint` _newestlane) :`1` _carspawnpoint2))
  (bind (_returnvalue_x _returnvalue_y _returnvalue_z) (`KismetMathLibrary.BreakVector` (`SceneComponent.K2_GetComponentLocation` _returnvalue)))
  (`self.SpawnCar` (`KismetMathLibrary.MakeVector` _returnvalue_x _returnvalue_y _returnvalue_z))
  (if (== _returnvalue _carspawnpoint2)
    (set `/Game/Blueprints/bp_cars.ForwardSpeed` -500.0 _newestcar)
    (else
      (set `/Game/Blueprints/bp_cars.ForwardSpeed` 500.0 _newestcar)))
  (set `/Game/Blueprints/bp_cars.StartPosition` (`KismetMathLibrary.MakeVector` _returnvalue_x _returnvalue_y _returnvalue_z) _newestcar))

(fn `SpawnCars`
  (bind _newestlane (`self.NewestLane`))
  (bind _returnvalue (* (`self.DefaultSpeed`) (`self.SpawnSpeed`)))
  (bind _returnvalue_2 (select `int` (`KismetMathLibrary.RandomIntegerInRange` 0 4) :`0` "/Game/vehicle/police_car.police_car" :`1` "/Game/vehicle/truck.truck" :`2` "/Game/vehicle/yellow_short_car.yellow_short_car" :`3` "/Game/vehicle/fedex.fedex" :!type "StaticMesh Object Reference"))
  (bind _returnvalue_3 (`SceneComponent.K2_GetComponentLocation` (`/Game/Blueprints/bp_lane.CarSpawnPoint2` _newestlane)))
  (bind _returnvalue_4 (`SceneComponent.K2_GetComponentLocation` (`/Game/Blueprints/bp_lane.CarSpawnPoint` _newestlane)))
  (bind _returnvalue_5 (== _returnvalue_2 "/Game/vehicle/truck.truck"))
  (set `self.DefaultSpeed` (`/Game/Blueprints/bp_lane.DefaultSpeed` _newestlane))
  (set `self.SpawnSpeed` (`/Game/Blueprints/bp_lane.SpawnSpeed` _newestlane))
  (if (== 1.0 (`/Game/Blueprints/bp_lane.SpawnDirection` _newestlane))
    (bind _returnvalue_6 (`|SpawnActorFromClass` "/Game/Blueprints/bp_cars.bp_cars_C" (`KismetMathLibrary.MakeTransform` _returnvalue_4) "Undefined" "OverrideRootScale" self null))
    (set `/Game/Blueprints/bp_cars.ForwardSpeed` _returnvalue _returnvalue_6)
    (bind _output_get (set `self.NewestCar` _returnvalue_6))
    (`StaticMeshComponent.SetStaticMesh` (`/Game/Blueprints/bp_cars.StaticMesh` _output_get) _returnvalue_2)
    (if _returnvalue_5
      (set `/Game/Blueprints/bp_cars.StartPosition` (+ _returnvalue_4 (0.0 0.0 300.0)) _output_get))
    (else
      (bind _returnvalue_7 (`|SpawnActorFromClass` "/Game/Blueprints/bp_cars.bp_cars_C" (`KismetMathLibrary.MakeTransform` _returnvalue_3 (struct :`Yaw` 180.0)) "Undefined" "OverrideRootScale" self null))
      (set `/Game/Blueprints/bp_cars.ForwardSpeed` (* -1.0 _returnvalue) _returnvalue_7)
      (bind _output_get_2 (set `self.NewestCar` _returnvalue_7))
      (`StaticMeshComponent.SetStaticMesh` (`/Game/Blueprints/bp_cars.StaticMesh` _output_get_2) _returnvalue_2)
      (if _returnvalue_5
        (set `/Game/Blueprints/bp_cars.StartPosition` (+ _returnvalue_3 (0.0 0.0 300.0)) _output_get_2)))))

(fn `SpawnInitialLanes`
  (bind _newestlane (`self.NewestLane`))
  (bind (_returnvalue_x _returnvalue_y) (`KismetMathLibrary.BreakVector` (`self.K2_GetActorLocation` (`GameplayStatics.GetPlayerPawn` 0))))
  (for _index (range 21)
    (set `self.InitialLaneNumber` _index)
    (`/Engine/EditorBlueprintResources/StandardMacros.IsValid` _newestlane
      (:`Is Valid`
        (`self.SpawnLaneAtSpawnPoint`)
        (`/Game/Blueprints/bp_lane.ManageSpawns` _newestlane))
      (:`Is Not Valid`
        (`self.SpawnLane` (`KismetMathLibrary.MakeVector` _returnvalue_x _returnvalue_y))))))

(fn `SpawnLane`
  (params (SpawnLocation :type "Vector Structure"))
  (bind _lanestate (`self.LaneState`))
  (bind (_startlocation_x _startlocation_y _startlocation_z) (`KismetMathLibrary.BreakVector` (`self.startlocation`)))
  (bind (_startlocation_x_2 _startlocation_y_2 _startlocation_z_2) (`KismetMathLibrary.BreakVector` (`self.startlocation`)))
  (bind _returnvalue_x (`KismetMathLibrary.BreakVector` (`self.K2_GetActorLocation` (`GameplayStatics.GetPlayerPawn` 0))))
  (bind _staticmesh (`StaticMeshComponent.StaticMesh` (`/Game/Blueprints/bp_lane.lane` (`self.NewestLane`))))
  (if (> (+ _returnvalue_x (`self.createBuffer`)) SpawnLocation_X)
    (bind _returnvalue (`|SpawnActorFromClass` "/Game/Blueprints/bp_lane.bp_lane_C" (`KismetMathLibrary.MakeTransform` (`KismetMathLibrary.MakeVector` SpawnLocation_X SpawnLocation_Y SpawnLocation_Z)) "Undefined" "OverrideRootScale" null null))
    (bind _output_get (set `self.NewestLane` _returnvalue))
    (set `/Game/Blueprints/bp_lane.LaneSpawner` self _output_get)
    (if (< (`self.InitialLaneNumber`) 6)
      (set `self.LaneState` 0)
      (else
        (set `self.LaneState` (`KismetMathLibrary.RandomIntegerInRange` 0 3))))
    (set `/Game/Blueprints/bp_lane.lane_state` _lanestate _output_get)
    (`/Game/Blueprints/bp_lane.ChangeLane` _output_get _lanestate (`self.prevLane`))
    (if (or (== _staticmesh "/Game/highway/1lane_highway.1lane_highway") (== _staticmesh "/Game/highway/1lane_highway_marked.1lane_highway_marked"))
      (set `self.prevLane` true)
      (else
        (set `self.prevLane` false)))
    (switch `int` _lanestate
      (:`0`
        (bind _rocktree2 (`/Game/Blueprints/bp_lane.rocktree2` _output_get))
        (bind _output_get_2 (set `self.startlocation` (`SceneComponent.K2_GetComponentLocation` _rocktree2)))
        (bind _rocktree1 (`/Game/Blueprints/bp_lane.rocktree1` _output_get))
        (bind _output_get_3 (set `self.endlocation` (`SceneComponent.K2_GetComponentLocation` _rocktree1)))
        (for _index (range (+ (`KismetMathLibrary.FTrunc` (/ (`KismetMathLibrary.Vector_Distance` _output_get_3 _output_get_2) 85.0)) 1))
          (if (> (`KismetMathLibrary.RandomFloat`) 0.95)
            (switch `int` (`KismetMathLibrary.RandomIntegerInRange` 0 2)
              (:`0`
                (bind _returnvalue_2 (`KismetMathLibrary.MakeVector` _startlocation_x (+ (* _index 90.0) (.y (`self.startlocation`))) _startlocation_z))
                (`|SpawnActorFromClass` "/Game/Blueprints/treeSpawner.treeSpawner_C" (`KismetMathLibrary.MakeTransform` _returnvalue_2) "Undefined" "OverrideRootScale" null null))
              (:`1`
                (`|SpawnActorFromClass` "/Game/Blueprints/rockSpawner.rockSpawner_C" (`KismetMathLibrary.MakeTransform` _returnvalue_2) "Undefined" "OverrideRootScale" null null))
              (:`2`
                (`|SpawnActorFromClass` "/Game/Blueprints/Coin.Coin_C" (`KismetMathLibrary.MakeTransform` _returnvalue_2) "Undefined" "OverrideRootScale" null null))))))
      (:`3`
        (bind _output_get_4 (set `self.startlocation` (`SceneComponent.K2_GetComponentLocation` _rocktree2)))
        (bind _output_get_5 (set `self.endlocation` (`SceneComponent.K2_GetComponentLocation` _rocktree1)))
        (for _index_2 (range (+ (`KismetMathLibrary.FTrunc` (/ (`KismetMathLibrary.Vector_Distance` _output_get_5 _output_get_4) 85.0)) 1))
          (if (> (`KismetMathLibrary.RandomFloat`) 0.98)
            (bind _returnvalue_3 (`KismetMathLibrary.MakeVector` _startlocation_x_2 (+ (* _index_2 90.0) (.y (`self.startlocation`))) _startlocation_z_2))
            (`|SpawnActorFromClass` "/Game/Blueprints/lilypadSpawner.lilypadSpawner_C" (`KismetMathLibrary.MakeTransform` _returnvalue_3) "Undefined" "OverrideRootScale" null null)
            (if (== (`KismetMathLibrary.RandomIntegerInRange` 0 5) 5)
              (`|SpawnActorFromClass` "/Game/Blueprints/Coin.Coin_C" (`KismetMathLibrary.MakeTransform` _returnvalue_3) "Undefined" "OverrideRootScale" null null))))))))

(fn `SpawnLaneAtSpawnPoint`
  (bind (_returnvalue_x _returnvalue_y _returnvalue_z) (`KismetMathLibrary.BreakVector` (`SceneComponent.K2_GetComponentLocation` (`/Game/Blueprints/bp_lane.SpawnPoint` (`self.NewestLane`)))))
  (`self.SpawnLane` (`KismetMathLibrary.MakeVector` _returnvalue_x _returnvalue_y _returnvalue_z)))

(fn `SpawnLog`
  (params (SpawnLocation :type "Vector Structure"))
  (bind _returnvalue (`|SpawnActorFromClass` "/Game/Blueprints/bp_log.bp_log_C" (`KismetMathLibrary.MakeTransform` SpawnLocation) "Undefined" "OverrideRootScale" null null))
  (bind _output_get (set `self.NewestLog` _returnvalue))
  (set `/Game/Blueprints/bp_log.LogSpawner` self _output_get))

(fn `SpawnLogAtSpawnPoint`
  (bind _newestlane (`self.NewestLane`))
  (bind _newestlog (`self.NewestLog`))
  (bind _carspawnpoint2 (`/Game/Blueprints/bp_lane.CarSpawnPoint2` _newestlane))
  (bind _returnvalue (select `int` (`KismetMathLibrary.RandomIntegerInRange` 0 1) :`0` (`/Game/Blueprints/bp_lane.CarSpawnPoint` _newestlane) :`1` _carspawnpoint2))
  (bind (_returnvalue_x _returnvalue_y _returnvalue_z) (`KismetMathLibrary.BreakVector` (`SceneComponent.K2_GetComponentLocation` _returnvalue)))
  (if (== _returnvalue _carspawnpoint2)
    (`self.SpawnLog` (`KismetMathLibrary.MakeVector` _returnvalue_x _returnvalue_y _returnvalue_z))
    (set `/Game/Blueprints/bp_log.ForwardSpeed` 500.0 _newestlog)
    (else
      (`self.SpawnLog` (`KismetMathLibrary.MakeVector` _returnvalue_x _returnvalue_y _returnvalue_z))
      (set `/Game/Blueprints/bp_log.ForwardSpeed` -500.0 _newestlog))))

(fn `SpawnLogs`
  (bind _newestlane (`self.NewestLane`))
  (bind _returnvalue (* (`self.DefaultSpeed`) (`self.SpawnSpeed`)))
  (set `self.DefaultSpeed` (`/Game/Blueprints/bp_lane.DefaultSpeed` _newestlane))
  (set `self.SpawnSpeed` (`/Game/Blueprints/bp_lane.SpawnSpeed` _newestlane))
  (if (== 1.0 (`/Game/Blueprints/bp_lane.SpawnDirection` _newestlane))
    (bind _returnvalue_2 (`|SpawnActorFromClass` "/Game/Blueprints/bp_log.bp_log_C" (`KismetMathLibrary.MakeTransform` (`SceneComponent.K2_GetComponentLocation` (`/Game/Blueprints/bp_lane.CarSpawnPoint` _newestlane))) "Undefined" "OverrideRootScale" self null))
    (set `/Game/Blueprints/bp_log.ForwardSpeed` _returnvalue _returnvalue_2)
    (else
      (bind _returnvalue_3 (`|SpawnActorFromClass` "/Game/Blueprints/bp_log.bp_log_C" (`KismetMathLibrary.MakeTransform` (`SceneComponent.K2_GetComponentLocation` (`/Game/Blueprints/bp_lane.CarSpawnPoint2` _newestlane))) "Undefined" "OverrideRootScale" self null))
      (set `/Game/Blueprints/bp_log.ForwardSpeed` (* -1.0 _returnvalue) _returnvalue_3))))

(fn `SpawnTrain`
  (params (SpawnLocation :type "Vector Structure"))
  (bind _returnvalue (`|SpawnActorFromClass` "/Game/Blueprints/bp_train.bp_train_C" (`KismetMathLibrary.MakeTransform` SpawnLocation) "Undefined" "OverrideRootScale" null null))
  (bind _output_get (set `self.NewestTrain` _returnvalue))
  (set `/Game/Blueprints/bp_train.TrainSpawner` self _output_get))

(fn `SpawnTrainAtSpawnPoint`
  (bind _newesttrain (`self.NewestTrain`))
  (bind _newestlane (`self.NewestLane`))
  (bind _carspawnpoint2 (`/Game/Blueprints/bp_lane.CarSpawnPoint2` _newestlane))
  (bind _returnvalue (select `int` (`KismetMathLibrary.RandomIntegerInRange` 0 1) :`0` (`/Game/Blueprints/bp_lane.CarSpawnPoint` _newestlane) :`1` _carspawnpoint2))
  (bind (_returnvalue_x _returnvalue_y _returnvalue_z) (`KismetMathLibrary.BreakVector` (`SceneComponent.K2_GetComponentLocation` _returnvalue)))
  (`self.SpawnTrain` (`KismetMathLibrary.MakeVector` _returnvalue_x _returnvalue_y _returnvalue_z))
  (if (== _returnvalue _carspawnpoint2)
    (set `/Game/Blueprints/bp_train.ForwardSpeed` -2000.0 _newesttrain)
    (else
      (set `/Game/Blueprints/bp_train.ForwardSpeed` 2000.0 _newesttrain))))

(fn `SpawnTrains`
  (bind _newestlane (`self.NewestLane`))
  (bind _returnvalue (* (`self.DefaultSpeed`) (`self.SpawnSpeed`)))
  (set `self.DefaultSpeed` (`/Game/Blueprints/bp_lane.DefaultSpeed` _newestlane))
  (set `self.SpawnSpeed` (`/Game/Blueprints/bp_lane.SpawnSpeed` _newestlane))
  (if (== 1.0 (`/Game/Blueprints/bp_lane.SpawnDirection` _newestlane))
    (bind _returnvalue_2 (`|SpawnActorFromClass` "/Game/Blueprints/bp_train.bp_train_C" (`KismetMathLibrary.MakeTransform` (`SceneComponent.K2_GetComponentLocation` (`/Game/Blueprints/bp_lane.CarSpawnPoint` _newestlane))) "Undefined" "OverrideRootScale" self null))
    (set `/Game/Blueprints/bp_train.ForwardSpeed` _returnvalue _returnvalue_2)
    (else
      (bind _returnvalue_3 (`|SpawnActorFromClass` "/Game/Blueprints/bp_train.bp_train_C" (`KismetMathLibrary.MakeTransform` (`SceneComponent.K2_GetComponentLocation` (`/Game/Blueprints/bp_lane.CarSpawnPoint2` _newestlane)) (struct :`Yaw` 180.0)) "Undefined" "OverrideRootScale" self null))
      (set `/Game/Blueprints/bp_train.ForwardSpeed` (* -1.0 _returnvalue) _returnvalue_3))))

(fn `timer`)

(fn `UserConstructionScript`)