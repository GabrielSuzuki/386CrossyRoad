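; Lane actor for a Crossy Road-style game, configured by ChangeLane as grass, highway, railroad or water, with randomized traffic direction and speed.
; A Tick-driven countdown spawns cars, trains or logs from either side, and end triggers destroy them.
; Player overlaps ask LaneSpawner for another lane or cause drowning on water.
; The lane destroys itself once the player's X plus a buffer exceeds its own.
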(event `self.ReceiveBeginPlay`
  (set `self.SpawnTimer` (`KismetMathLibrary.RandomIntegerInRange` 100 500)))

(event `self.ReceiveTick`
  (params (DeltaSeconds :type "Float (single-precision)"))
  (bind _returnvalue_x (`KismetMathLibrary.BreakVector` (`self.K2_GetActorLocation`)))
  (bind _returnvalue_x_2 (`KismetMathLibrary.BreakVector` (`self.K2_GetActorLocation` (`GameplayStatics.GetPlayerPawn` 0))))
  (`self.ManageSpawns`)
  (if (> (+ _returnvalue_x_2 (`self.DestroyBuffer`)) _returnvalue_x)
    (`self.K2_DestroyActor`)))

(event `self.TriggerZone.OnComponentBeginOverlap`
  (params (OverlappedComponent :type "PrimitiveComponent Object Reference") (OtherActor :type "Actor Object Reference") (OtherComp :type "PrimitiveComponent Object Reference") (OtherBodyIndex :type Integer) (bFromSweep :type Boolean) (SweepResult :type "HitResult Structure (by ref)"))
  (cast `/Game/Blueprints/ThirdPersonCharacter` OtherActor)
  (`/Game/Blueprints/bp_lane_spawner.SpawnLaneAtSpawnPoint` (`self.LaneSpawner`)))

(event `MovementCooldown`
  (`/Engine/EditorBlueprintResources/StandardMacros.DoOnce` false :!label _label
    (:`Completed`
      (set `self.canmove` false)
      (`KismetSystemLibrary.Delay` 0.5)
      (set `self.canmove` true)
      (goto _label :!via `Reset`))))

(event `self.CarTriggerZone1.OnComponentBeginOverlap`
  (params (OverlappedComponent :type "PrimitiveComponent Object Reference") (OtherActor :type "Actor Object Reference") (OtherComp :type "PrimitiveComponent Object Reference") (OtherBodyIndex :type Integer) (bFromSweep :type Boolean) (SweepResult :type "HitResult Structure (by ref)"))
  (bind _asbp_cars (cast `/Game/Blueprints/bp_cars` OtherActor)
    (:`then`
      (`self.K2_DestroyActor` _asbp_cars))
    (:`CastFailed`
      (bind _asbp_train (cast `/Game/Blueprints/bp_train` OtherActor)
        (:`then`
          (`self.K2_DestroyActor` _asbp_train))
        (:`CastFailed`
          (bind _asbp_log (cast `/Game/Blueprints/bp_log` OtherActor))
          (`self.K2_DestroyActor` _asbp_log)))))
  (`self.ManageSpawns` :!label _label_2))

(event `self.CarTriggerZone2.OnComponentBeginOverlap`
  (params (OverlappedComponent :type "PrimitiveComponent Object Reference") (OtherActor :type "Actor Object Reference") (OtherComp :type "PrimitiveComponent Object Reference") (OtherBodyIndex :type Integer) (bFromSweep :type Boolean) (SweepResult :type "HitResult Structure (by ref)"))
  (bind _asbp_cars (cast `/Game/Blueprints/bp_cars` OtherActor)
    (:`then`
      (`self.K2_DestroyActor` _asbp_cars)
      (goto _label_2))
    (:`CastFailed`
      (bind _asbp_train (cast `/Game/Blueprints/bp_train` OtherActor)
        (:`then`
          (`self.K2_DestroyActor` _asbp_train)
          (goto _label_2))
        (:`CastFailed`
          (bind _asbp_log (cast `/Game/Blueprints/bp_log` OtherActor))
          (`self.K2_DestroyActor` _asbp_log)
          (goto _label_2))))))

(event `self.WaterTriggerZone.OnComponentBeginOverlap`
  (params (OverlappedComponent :type "PrimitiveComponent Object Reference") (OtherActor :type "Actor Object Reference") (OtherComp :type "PrimitiveComponent Object Reference") (OtherBodyIndex :type Integer) (bFromSweep :type Boolean) (SweepResult :type "HitResult Structure (by ref)"))
  (bind _asthird_person_character (cast `/Game/Blueprints/ThirdPersonCharacter` OtherActor))
  (if (== (`self.lane_state`) 3)
    (`/Game/Blueprints/ThirdPersonCharacter.Drowned` _asthird_person_character)))

(fn `ChangeLane`
  (params (`Lane Type` :type Integer) (prevlane :type Boolean))
  (bind _lane (`self.lane`))
  (set `self.previousLaneIsHighway` prevlane)
  (bind _output_get (set `self.lane_state` `Lane Type`))
  (bind _returnvalue (select `int` _output_get :`0` "/Game/grass/1lane_grass.1lane_grass" :`1` "/Game/highway/1lane_highway.1lane_highway" :`2` "/Game/railroad/railroad.railroad" :`3` "/Game/water/1lane_water_vox.1lane_water_vox" :!type "StaticMesh Object Reference"))
  (if (and (== _returnvalue "/Game/highway/1lane_highway.1lane_highway") (`self.previousLaneIsHighway`))
    (`StaticMeshComponent.SetStaticMesh` _lane "/Game/highway/1lane_highway_marked.1lane_highway_marked")
    (else
      (`StaticMeshComponent.SetStaticMesh` _lane _returnvalue)))
  (if (`KismetMathLibrary.RandomBool`)
    (set `self.SpawnDirection` 1.0)
    (else
      (set `self.SpawnDirection` -1.0)))
  (switch `int` (`self.lane_state`)
    (:`1`
      (bind _output_get_2 (set `self.SpawnType` (`KismetMathLibrary.RandomIntegerInRange` 0 3)))
      (set `self.DefaultSpeed` 400.0)
      (set `self.SpawnSpeed` (`KismetMathLibrary.RandomFloatInRange` (select `int` _output_get_2 :`0` 2.5 :`1` 1.0 :`2` 1.0 :!type "Float (single-precision)") (select `int` _output_get_2 :`0` 5.0 :`1` 6.0 :`2` 3.0 :`3` 2.0 :!type "Float (single-precision)"))))
    (:`2`
      (set `self.DefaultSpeed` 2000.0)
      (set `self.SpawnTimer` (* (`KismetMathLibrary.RandomIntegerInRange` 5 15) 130)))
    (:`3`
      (`SceneComponent.SetWorldScale3D` (`self.lane`) (100.0 100.0 100.0))
      (`SceneComponent.K2_SetWorldRotation` (`self.lane`) (struct :`Roll` 90.0) false false)
      (bind _output_get_3 (set `self.SpawnType` (`KismetMathLibrary.RandomIntegerInRange` 0 3)))
      (set `self.DefaultSpeed` 400.0)
      (set `self.SpawnSpeed` (`KismetMathLibrary.RandomFloatInRange` 1.0 1.75))
      (if (== _output_get_3 0)
        _))))

(fn `ManageSpawns`
  (locals (SpawnTimerLocal :type Integer))
  (bind _result (`/Engine/EditorBlueprintResources/StandardMacros.DecrementInt` (`self.SpawnTimer`))
    (:`  `
      (if (<= _result 0)
        (switch `int` (`self.lane_state`)
          (:`0`
            (set `self.SpawnTimer` 100))
          (:`1`
            (bind _asbp_cars (castclass `/Game/Blueprints/bp_cars` "/Game/Blueprints/bp_cars.bp_cars_C"))
            (set `self.ToBeSpawned` _asbp_cars)
            (`self.SpawnMoving`))
          (:`2`
            (bind _asbp_train (castclass `/Game/Blueprints/bp_train` "/Game/Blueprints/bp_train.bp_train_C"))
            (set `self.ToBeSpawned` _asbp_train)
            (`self.SpawnMoving`)
            (`GameplayStatics.PlaySound2D` "/Game/Sounds/166086__felix-blume__train-passing-by-in-the-wirikuta-desert-mexico-slp.166086__felix-blume__train-passing-by-in-the-wirikuta-desert-mexico-slp" 0.2 1.0 0.0 null null))
          (:`3`
            (bind _asbp_log (castclass `/Game/Blueprints/bp_log` "/Game/Blueprints/bp_log.bp_log_C"))
            (set `self.ToBeSpawned` _asbp_log)
            (`self.SpawnMoving`)))))))

(fn `SpawnMoving`
  (bind _carspawnpoint2 (`self.CarSpawnPoint2`))
  (bind _objectspeed (`self.ObjectSpeed`))
  (bind (_returnvalue_x _returnvalue_y _returnvalue_z) (`KismetMathLibrary.BreakVector` (`SceneComponent.K2_GetComponentLocation` (`self.CurrentSpawner`))))
  (bind _returnvalue (== _carspawnpoint2 (`self.CurrentSpawner`)))
  (bind _returnvalue_2 (* (`self.DefaultSpeed`) (`self.SpawnSpeed`)))
  (if (== 1.0 (`self.SpawnDirection`))
    (set `self.CurrentSpawner` (`self.CarSpawnPoint`))
    (else
      (set `self.CurrentSpawner` _carspawnpoint2)))
  (bind _returnvalue_3 (`|SpawnActorFromClass` (`self.ToBeSpawned`) (`KismetMathLibrary.MakeTransform` (`KismetMathLibrary.MakeVector` _returnvalue_x (+ (`self.offset`) _returnvalue_y) _returnvalue_z)) "Undefined" "OverrideRootScale" self null))
  (if _returnvalue
    (set `self.ObjectSpeed` (* -1.0 _returnvalue_2))
    (else
      (set `self.ObjectSpeed` _returnvalue_2)))
  (bind _asbp_cars (cast `/Game/Blueprints/bp_cars` _returnvalue_3)
    (:`then`
      (set `/Game/Blueprints/bp_cars.ForwardSpeed` _objectspeed _asbp_cars)
      (set `self.SpawnTimer` (* (`KismetMathLibrary.RandomIntegerInRange` 1 10) (`KismetMathLibrary.FTrunc` (/ (select `int` (`self.SpawnType`) :`0` 210.0 :`1` 150.0 :`2` 120.0 :`3` 120.0 :!type "Float (single-precision)") (`self.SpawnSpeed`)))))
      (if _returnvalue
        (`self.K2_SetActorRelativeRotation` _asbp_cars (struct :`Yaw` 180.0) false false)))
    (:`CastFailed`
      (bind _asbp_train (cast `/Game/Blueprints/bp_train` _returnvalue_3)
        (:`then`
          (set `/Game/Blueprints/bp_train.ForwardSpeed` _objectspeed _asbp_train)
          (set `self.SpawnTimer` (* (`KismetMathLibrary.RandomIntegerInRange` 5 15) 130))
          (if _returnvalue
            (`self.K2_SetActorRelativeRotation` _asbp_train (struct :`Yaw` 180.0) false false)))
        (:`CastFailed`
          (bind _asbp_log (cast `/Game/Blueprints/bp_log` _returnvalue_3))
          (set `/Game/Blueprints/bp_log.ForwardSpeed` _objectspeed _asbp_log)
          (set `self.SpawnTimer` (`KismetMathLibrary.FTrunc` (/ (`KismetMathLibrary.Conv_IntToDouble` (* (`KismetMathLibrary.RandomIntegerInRange` 1 3) 200)) (`self.SpawnSpeed`))))
          (if _returnvalue
            (`self.K2_SetActorRelativeRotation` _asbp_log (struct :`Yaw` 180.0) false false)))))))

(fn `UserConstructionScript`)