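; Eagle actor that descends on a timeline and can catch the third-person character, pinning it just above itself.
; BeginPlay lerps its height down from Startlocation and latches Enable late in the timeline.
; A Box overlap stores the character and sets Hit.
; Once both flags are true, Tick snaps the character above the eagle every frame, with neither flag ever reset.
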(event `self.ReceiveTick`
  (params (DeltaSeconds :type "Float (single-precision)"))
  (bind (_returnvalue_x _returnvalue_y _returnvalue_z) (`KismetMathLibrary.BreakVector` (`self.K2_GetActorLocation`)))
  (if (`self.enable`)
    (if (`self.Hit`)
      (`self.K2_SetActorLocation` (`self.thirdpersonchar`) (`KismetMathLibrary.MakeVector` _returnvalue_x _returnvalue_y (+ _returnvalue_z 100.0)) false false))))

(event `self.ReceiveBeginPlay`
  (bind (_startlocation_x _startlocation_y _startlocation_z) (`KismetMathLibrary.BreakVector` (`self.startlocation`)))
  (bind (_startlocation_x_2 _startlocation_y_2 _startlocation_z_2) (`KismetMathLibrary.BreakVector` (`self.startlocation`)))
  (set `self.endlocation` (+ _startlocation_z_2 -90.0))
  (bind (_direction _newtrack_0) (`Timeline|Timeline_0` :!via `PlayFromStart`)
    (:`Update`
      (`self.K2_SetActorLocation` (`KismetMathLibrary.MakeVector` _startlocation_x _startlocation_y (`KismetMathLibrary.Lerp` _startlocation_z (`self.endlocation`) _newtrack_0)))
      (if (not (`self.enable`))
        (set `self.enable` (and (> _newtrack_0 0.7) (> 1.0 _newtrack_0)))))))

(event `self.Box.OnComponentBeginOverlap`
  (params (OverlappedComponent :type "PrimitiveComponent Object Reference") (OtherActor :type "Actor Object Reference") (OtherComp :type "PrimitiveComponent Object Reference") (OtherBodyIndex :type Integer) (bFromSweep :type Boolean) (SweepResult :type "HitResult Structure (by ref)"))
  (bind _asthird_person_character (cast `/Game/Blueprints/ThirdPersonCharacter` OtherActor))
  (set `self.thirdpersonchar` _asthird_person_character)
  (set `self.Hit` true))

(fn `UserConstructionScript`)