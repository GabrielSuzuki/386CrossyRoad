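; bp_cars is a vehicle obstacle that gets a random car mesh at BeginPlay and can hit the player.
; Each Tick moves it along world Y at ForwardSpeed, or destroys it once the player's X plus DestroyBuffer passes its X.
; Box overlaps ignore bp_lane and call HitByVechile on ThirdPersonCharacter when their X offset is nonzero but small.
; The travel-distance check leads nowhere, and the squash and position-reset nodes are disconnected.
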(event `self.ReceiveBeginPlay`
  (set `self.StartPosition` (`self.K2_GetActorLocation`))
  (`StaticMeshComponent.SetStaticMesh` (`self.StaticMesh`) (select `int` (`KismetMathLibrary.RandomIntegerInRange` 0 3) :`0` "/Game/vehicle/police_car.police_car" :`1` "/Game/vehicle/red_car.red_car" :`2` "/Game/vehicle/fedex.fedex" :`3` "/Game/vehicle/yellow_short_car.yellow_short_car" :!type "StaticMesh Object Reference")))

(event `self.ReceiveTick`
  (params (DeltaSeconds :type "Float (single-precision)"))
  (bind _returnvalue_x (`KismetMathLibrary.BreakVector` (`self.K2_GetActorLocation`)))
  (bind _returnvalue_x_2 (`KismetMathLibrary.BreakVector` (`self.K2_GetActorLocation` (`GameplayStatics.GetPlayerPawn` 0))))
  (if (> (+ _returnvalue_x_2 (`self.DestroyBuffer`)) _returnvalue_x)
    (`self.K2_DestroyActor`)
    (else
      (`self.K2_AddActorWorldOffset` (`KismetMathLibrary.MakeVector` 0.0 (* DeltaSeconds (`self.ForwardSpeed`))))
      (if (> (`KismetMathLibrary.Vector_Distance` (`self.K2_GetActorLocation`) (`self.StartPosition`)) (`self.Distance`))
        _))))

(event `self.Box.OnComponentBeginOverlap`
  (params (OverlappedComponent :type "PrimitiveComponent Object Reference") (OtherActor :type "Actor Object Reference") (OtherComp :type "PrimitiveComponent Object Reference") (OtherBodyIndex :type Integer) (bFromSweep :type Boolean) (SweepResult :type "HitResult Structure (by ref)"))
  (bind _returnvalue_x (`KismetMathLibrary.BreakVector` (`self.K2_GetActorLocation`)))
  (cast `/Game/Blueprints/bp_lane` OtherActor
    (:`CastFailed`
      (bind _asthird_person_character (cast `/Game/Blueprints/ThirdPersonCharacter` OtherActor))
      (bind _returnvalue_x_2 (`KismetMathLibrary.BreakVector` (`self.K2_GetActorLocation` _asthird_person_character)))
      (bind _returnvalue (`KismetMathLibrary.Abs` (- _returnvalue_x _returnvalue_x_2)))
      (if (and (> _returnvalue 0.0) (< _returnvalue 5.0))
        (`/Game/Blueprints/ThirdPersonCharacter.HitByVechile` _asthird_person_character)))))

(fn `UserConstructionScript`)