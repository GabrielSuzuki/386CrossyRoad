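; Train hazard that crosses along Y and hits the player's ThirdPersonCharacter.
; BeginPlay picks one of two train meshes at random; Tick moves it at ForwardSpeed, snapping back to its start beyond Distance.
; It destroys itself once player X plus DestroyBuffer exceeds its own X.
; Box overlap calls HitByVechile only for a nonzero X offset under five units; Box1's train overlap does nothing after the cast.
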(event `self.ReceiveBeginPlay`
  (set `self.StartPosition` (`self.K2_GetActorLocation`))
  (`StaticMeshComponent.SetStaticMesh` (`self.StaticMesh`) (select `int` (`KismetMathLibrary.RandomIntegerInRange` 0 1) :`0` "/Game/vehicle/train_5.train_5" :`1` "/Game/vehicle/train_6.train_6" :!type "StaticMesh Object Reference")))

(event `self.ReceiveTick`
  (params (DeltaSeconds :type "Float (single-precision)"))
  (bind _returnvalue_x (`KismetMathLibrary.BreakVector` (`self.K2_GetActorLocation`)))
  (bind _returnvalue_x_2 (`KismetMathLibrary.BreakVector` (`self.K2_GetActorLocation` (`GameplayStatics.GetPlayerPawn` 0))))
  (if (> (+ _returnvalue_x_2 (`self.DestroyBuffer`)) _returnvalue_x)
    (`self.K2_DestroyActor`)
    (else
      (`self.K2_AddActorWorldOffset` (`KismetMathLibrary.MakeVector` 0.0 (* DeltaSeconds (`self.ForwardSpeed`))))
      (if (> (`KismetMathLibrary.Vector_Distance` (`self.K2_GetActorLocation`) (`self.StartPosition`)) (`self.Distance`))
        (`self.K2_SetActorLocation` (`self.StartPosition`))))))

(event `self.Box.OnComponentBeginOverlap`
  (params (OverlappedComponent :type "PrimitiveComponent Object Reference") (OtherActor :type "Actor Object Reference") (OtherComp :type "PrimitiveComponent Object Reference") (OtherBodyIndex :type Integer) (bFromSweep :type Boolean) (SweepResult :type "HitResult Structure (by ref)"))
  (bind _returnvalue_x (`KismetMathLibrary.BreakVector` (`self.K2_GetActorLocation`)))
  (bind _asthird_person_character (cast `/Game/Blueprints/ThirdPersonCharacter` OtherActor))
  (bind _returnvalue_x_2 (`KismetMathLibrary.BreakVector` (`self.K2_GetActorLocation` _asthird_person_character)))
  (bind _returnvalue (`KismetMathLibrary.Abs` (- _returnvalue_x _returnvalue_x_2)))
  (if (and (> _returnvalue 0.0) (< _returnvalue 5.0))
    (`/Game/Blueprints/ThirdPersonCharacter.HitByVechile` _asthird_person_character)))

(event `self.Box1.OnComponentBeginOverlap`
  (params (OverlappedComponent :type "PrimitiveComponent Object Reference") (OtherActor :type "Actor Object Reference") (OtherComp :type "PrimitiveComponent Object Reference") (OtherBodyIndex :type Integer) (bFromSweep :type Boolean) (SweepResult :type "HitResult Structure (by ref)"))
  (cast `/Game/Blueprints/bp_train` OtherActor))

(fn `UserConstructionScript`)