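; Coin pickup actor that raises the ThirdPersonCharacter's score when collected.
; On box overlap with that character, it increments the Score, destroys itself and plays a 2D coin sound.
; Each Tick it spins its root by a fixed, frame-rate-dependent step.
; Tick also destroys the coin once the player's X plus DestroyBuffer exceeds the coin's X, clearing coins along the X axis.
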(event `self.ReceiveTick`
  (params (DeltaSeconds :type "Float (single-precision)"))
  (bind _returnvalue_x (`KismetMathLibrary.BreakVector` (`self.K2_GetActorLocation`)))
  (bind _returnvalue_x_2 (`KismetMathLibrary.BreakVector` (`self.K2_GetActorLocation` (`GameplayStatics.GetPlayerPawn` 0))))
  (`SceneComponent.K2_AddLocalRotation` (`self.DefaultSceneRoot`) (struct :`Yaw` 1.0) false false)
  (if (> (+ _returnvalue_x_2 (`self.DestroyBuffer`)) _returnvalue_x)
    (`self.K2_DestroyActor`)))

(event `self.Box.OnComponentBeginOverlap`
  (params (OverlappedComponent :type "PrimitiveComponent Object Reference") (OtherActor :type "Actor Object Reference") (OtherComp :type "PrimitiveComponent Object Reference") (OtherBodyIndex :type Integer) (bFromSweep :type Boolean) (SweepResult :type "HitResult Structure (by ref)"))
  (bind _asthird_person_character (cast `/Game/Blueprints/ThirdPersonCharacter` OtherActor))
  (bind _result (`/Engine/EditorBlueprintResources/StandardMacros.IncrementInt` (`KismetMathLibrary.FTrunc` (`/Game/Blueprints/ThirdPersonCharacter.score` _asthird_person_character)))
    (:`  `
      (set `/Game/Blueprints/ThirdPersonCharacter.score` (`KismetMathLibrary.Conv_IntToDouble` _result) _asthird_person_character)
      (`self.K2_DestroyActor`)
      (`GameplayStatics.PlaySound2D` "/Game/Sounds/415083__harrietniamh__video-game-coin.415083__harrietniamh__video-game-coin" 0.7 1.0 0.0 null null))))

(fn `UserConstructionScript`)